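; BP_WeaponBase is a base weapon Blueprint that handles the cosmetic side of firing.
; FireLocal runs Animations, VFX and Shell in turn.
; It plays fire montages on the weapon mesh and the character's first-person mesh, then spawns a muzzle flash attached to AttackForward.
; After a delay, Shell spawns a shell actor at ShellForward and ejects it with a force along that component's forward vector.
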(event `self.FireLocal`
  (bind _shellforward (`self.ShellForward`))
  (`|PlayMontage` (`self.WeaponMesh`) (`self.FirstPersonPoseFire`)
    (:`then`
      (`|PlayMontage` (`FPSGameCharacter.Mesh1P` (`self.Character`)) (`self.FirstPersonCharacterPoseFire`)
        (:`then`
          (`GameplayStatics.SpawnEmitterAttached` (`self.MuzzleFlash`) (`self.AttackForward`))
          (`KismetSystemLibrary.Delay` (`self.ShellDelay`))
          (bind _returnvalue (`|SpawnActorFromClass` (`self.ShellClass`) (`KismetMathLibrary.MakeTransform` (`SceneComponent.K2_GetComponentLocation` _shellforward) (`SceneComponent.K2_GetComponentRotation` _shellforward)) "Undefined" "MultiplyWithRoot" null null))
          (bind _asbullet_shell (cast `BulletShell` _returnvalue))
          (`PrimitiveComponent.AddForce` (`BulletShell.BulletMesh` _asbullet_shell) (* (`SceneComponent.GetForwardVector` (`self.ShellForward`)) (`self.ShellEjectVelocity`)) "None" false))))))

(fn `UserConstructionScript`)